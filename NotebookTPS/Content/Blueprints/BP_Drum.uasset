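; BP_Drum is a destructible drum actor that explodes when its health runs out and leaves a chick behind.
; AnyDamage subtracts the damage from HP and prints the remaining value to the screen.
; At zero or below, it spawns a simple Niagara explosion and a BP_Chick at its location, then destroys itself.
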(event `self.ReceiveAnyDamage`
  (params (Damage :type "Float (single-precision)") (DamageType :type "DamageType Object Reference") (InstigatedBy :type "Controller Object Reference") (DamageCauser :type "Actor Object Reference"))
  (bind _returnvalue (`self.K2_GetActorLocation`))
  (`|ExecutionSequence`
    (:`then_0`
      (set `self.HP` (- (`self.HP`) Damage)))
    (:`then_1`
      (`KismetSystemLibrary.PrintString` (`KismetStringLibrary.BuildString_Double` "" "HP = " (`self.HP`))))
    (:`then_2`
      (if (<= (`self.HP`) 0.0)
        (`NiagaraFunctionLibrary.SpawnSystemAtLocation` "/Game/FX/NS_ExplosionSimple.NS_ExplosionSimple" _returnvalue)
        (`|SpawnActorFromClass` "/Game/Blueprints/BP_Chick.BP_Chick_C" (`KismetMathLibrary.Conv_VectorToTransform` _returnvalue) "Undefined" "MultiplyWithRoot" null null)
        (`self.K2_DestroyActor`)))))

(fn `UserConstructionScript`)