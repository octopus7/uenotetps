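; Player character with Enhanced Input move, look, jump and timeline FOV zoom, carrying a spawned MicroUzi on its Weapon socket.
; Fire spawns a ball FireDistance out from the muzzle, or a seven-way yaw fan with MultiShot, plus ejected shell casings and debug shapes.
; While fire is held, Tick repeats shots at FiringRate and always draws an aim line.
; Radial damage lowers HP, showing only debug death text at zero.
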(event `self.ReceiveBeginPlay`
  (bind _asplayer_controller (cast `PlayerController` (`self.GetController`)))
  (`EnhancedInputSubsystemInterface.AddMappingContext` (pcsubsystem `EnhancedInputLocalPlayerSubsystem` _asplayer_controller) "/Game/Input/IMC_Simple.IMC_Simple" 0 (struct))
  (bind _returnvalue (`|SpawnActorFromClass` "/Game/Blueprints/BP_MicroUzi.BP_MicroUzi_C" (`self.GetTransform`) "Undefined" "MultiplyWithRoot" null null))
  (`self.K2_AttachToComponent` _returnvalue (`self.Mesh`) "Weapon" "SnapToTarget" "SnapToTarget" "KeepRelative" true))

(event `EnhancedInput|/Game/Input/IA_Move`
  (params (ActionValue :type "Vector2D Structure") (ElapsedSeconds :type "Float (double-precision)") (TriggeredSeconds :type "Float (double-precision)") (InputAction :type "InputAction Object Reference" :default "/Game/Input/IA_Move.IA_Move"))
  (bind (_x _y) (`KismetMathLibrary.BreakVector2D` ActionValue))
  (bind (_returnvalue_roll _returnvalue_pitch _returnvalue_yaw) (`KismetMathLibrary.BreakRotator` (`self.GetControlRotation`)))
  (bind _returnvalue (`KismetMathLibrary.MakeRotator` 0.0 0.0 _returnvalue_yaw))
  (:`Triggered`
    (`self.AddMovementInput` (+ (* (`KismetMathLibrary.GetForwardVector` _returnvalue) _y) (* (`KismetMathLibrary.GetRightVector` _returnvalue) _x)))))

(event `EnhancedInput|/Game/Input/IA_Look`
  (params (ActionValue :type "Vector2D Structure") (ElapsedSeconds :type "Float (double-precision)") (TriggeredSeconds :type "Float (double-precision)") (InputAction :type "InputAction Object Reference" :default "/Game/Input/IA_Look.IA_Look"))
  (:`Triggered`
    (`self.AddControllerPitchInput` ActionValue_Y)
    (`self.AddControllerYawInput` ActionValue_X)))

(event `EnhancedInput|/Game/Input/IA_Jump`
  (params (ActionValue :type Boolean) (ElapsedSeconds :type "Float (double-precision)") (TriggeredSeconds :type "Float (double-precision)") (InputAction :type "InputAction Object Reference" :default "/Game/Input/IA_Jump.IA_Jump"))
  (:`Started`
    (`self.Jump`)))

(event `EnhancedInput|/Game/Input/IA_Fire`
  (params (ActionValue :type Boolean) (ElapsedSeconds :type "Float (double-precision)") (TriggeredSeconds :type "Float (double-precision)") (InputAction :type "InputAction Object Reference" :default "/Game/Input/IA_Fire.IA_Fire"))
  (bind (_returnvalue_location _returnvalue_rotation) (`KismetMathLibrary.BreakTransform` (`SceneComponent.GetSocketTransform` (`self.Mesh`) "Muzzle" "RTS_World")))
  (:`Triggered`
    (set `self.IsFiring` true))
  (:`Started`
    (`|ExecutionSequence`
      (:`then_0`
        (if (`self.MultiShot`) :!label _label
          (for _index (range -3 4)
            (bind _returnvalue (`self.NewFunction` self _index))
            (`|ExecutionSequence` :!label _label_2
              (:`then_0`
                (`|SpawnActorFromClass` "/Game/Blueprints/BP_Ball.BP_Ball_C" (`KismetMathLibrary.MakeTransform` (stale _returnvalue_3) (stale _returnvalue2)) "Undefined" "MultiplyWithRoot" null null)
                (bind _returnvalue_2 (`|SpawnActorFromClass` "/Game/Blueprints/BP_ShellCasing.BP_ShellCasing_C" (`KismetMathLibrary.MakeTransform` (- _returnvalue_location (50.0 0.0 0.0)) _returnvalue_rotation) "Undefined" "MultiplyWithRoot" null null))
                (`PrimitiveComponent.AddForce` (`/Game/Blueprints/BP_ShellCasing.Cylinder` _returnvalue_2) (+ (* (`KismetMathLibrary.GetRightVector` _returnvalue_rotation) 1000.0) (* (`KismetMathLibrary.GetUpVector` _returnvalue_rotation) 200.0)) "None" false))
              (:`then_1`
                (`self.DrawDebugFunction` (stale _returnvalue_3) _returnvalue))))
          (else
            (bind (_returnvalue_3 _returnvalue2) (`self.NewFunction` self 0))
            (goto _label_2))))))
  (:`Completed`
    (set `self.IsFiring` false)))

(event `EnhancedInput|/Game/Input/IA_Zoom`
  (params (ActionValue :type Boolean) (ElapsedSeconds :type "Float (double-precision)") (TriggeredSeconds :type "Float (double-precision)") (InputAction :type "InputAction Object Reference" :default "/Game/Input/IA_Zoom.IA_Zoom"))
  (:`Started`
    (bind (_direction _fov) (`Timeline|Timeline` :!label _label_3)
      (:`Update`
        (`CameraComponent.SetFieldOfView` (`self.Camera`) _fov))))
  (:`Completed`
    (goto _label_3 :!via `Reverse`)))

(event `self.ReceiveTick`
  (params (DeltaSeconds :type "Float (single-precision)"))
  (bind (_returnvalue_location _returnvalue_rotation) (`KismetMathLibrary.BreakTransform` (`SceneComponent.GetSocketTransform` (`self.Mesh`) "Muzzle" "RTS_World")))
  (`|ExecutionSequence`
    (:`then_0`
      (`KismetSystemLibrary.DrawDebugLine` _returnvalue_location (+ _returnvalue_location (* (`KismetMathLibrary.GetForwardVector` _returnvalue_rotation) 3000.0)) (struct :`R` 1.0 :`B` 0.353911 :`A` 1.0)))
    (:`then_1`
      (if (`self.IsFiring`)
        (set `self.ElapsedTimeSinceFire` (+ (`self.ElapsedTimeSinceFire`) DeltaSeconds))
        (if (> (`self.ElapsedTimeSinceFire`) (`self.FiringRate`))
          (set `self.ElapsedTimeSinceFire` (- (`self.ElapsedTimeSinceFire`) (`self.FiringRate`)))
          (goto _label))))))

(event `self.ReceiveRadialDamage`
  (params (DamageReceived :type "Float (single-precision)") (DamageType :type "DamageType Object Reference") (Origin :type "Vector Structure") (HitInfo :type "HitResult Structure (by ref)") (InstigatedBy :type "Controller Object Reference") (DamageCauser :type "Actor Object Reference"))
  (bind _output_get (set `self.HP` (`KismetMathLibrary.FTrunc` (- (`self.HP`) DamageReceived))))
  (if (<= _output_get 0)
    (`KismetSystemLibrary.DrawDebugString` (`self.K2_GetActorLocation`) "YOU DIED" null (struct :`R` 1.0 :`G` 1.0 :`B` 1.0 :`A` 1.0) 5.0)))

(fn `AddChicken`
  (params (Count :type Integer) (HP :type Integer))
  (bind _output_get (set `self.ChickenCount` (+ Count (`self.ChickenCount`))))
  (bind _output_get_2 (set `self.HP` (+ (`self.HP`) HP)))
  (`KismetSystemLibrary.PrintString` (`KismetStringLibrary.Concat_StrStr` (`KismetStringLibrary.Concat_StrStr` "chicken count :" (`KismetStringLibrary.Conv_IntToString` _output_get)) (`KismetStringLibrary.Concat_StrStr` " hp :" (`KismetStringLibrary.Conv_IntToString` _output_get_2)))))

(fn `DrawDebugFunction`
  (params (LineEnd :type "Vector Structure") (Center :type "Vector Structure"))
  (`KismetSystemLibrary.DrawDebugSphere` Center 10.0 8 (struct :`R` 1.0 :`G` 1.0 :`B` 1.0 :`A` 1.0) 4.0)
  (`KismetSystemLibrary.DrawDebugLine` (`SceneComponent.GetSocketLocation` (`self.Mesh`) "Muzzle") LineEnd (struct :`R` 1.0 :`G` 0.464954 :`A` 1.0) 4.0))

(fn `GetFirePos`
  (params (target :type "SceneComponent Object Reference"))
  (returns (ReturnValue :type "Vector Structure"))
  (return (+ (`SceneComponent.GetSocketLocation` target "Muzzle") (* (`KismetMathLibrary.GreaterGreater_VectorRotator` (`KismetMathLibrary.Vector_Forward`) (`SceneComponent.GetSocketRotation` (`self.Mesh`) "Muzzle")) (`self.FireDistance`)))))

(fn `NewFunction`
  (params (InInt :type Integer))
  (returns (ReturnValue :type "Vector Structure") (ReturnValue2 :type "Rotator Structure"))
  (bind _mesh (`self.Mesh`))
  (bind _returnvalue (`KismetMathLibrary.ComposeRotators` (`KismetMathLibrary.MakeRotator` 0.0 0.0 (* (`KismetMathLibrary.Conv_IntToDouble` InInt) 20.0)) (`SceneComponent.GetSocketRotation` _mesh "Muzzle")))
  (return (+ (`SceneComponent.GetSocketLocation` _mesh "Muzzle") (* (`KismetMathLibrary.GreaterGreater_VectorRotator` (`KismetMathLibrary.Vector_Forward`) _returnvalue) (`self.FireDistance`))) _returnvalue))

(fn `UserConstructionScript`)