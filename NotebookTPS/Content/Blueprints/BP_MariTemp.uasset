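; BP_MariTemp is a character Blueprint, apparently temporary, with a radial attack and a capsule that grows whenever it takes damage.
; TryAttack applies radial damage around the actor when AttackCooltime has expired and draws a red debug sphere of that radius.
; It then calls SetAttackCooltime, whose body is empty here, so this file never starts the cooldown.
; UpdateWalkSpeed sets the movement component's maximum walk speed.
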(event `self.ReceiveAnyDamage`
  (params (Damage :type "Float (single-precision)") (DamageType :type "DamageType Object Reference") (InstigatedBy :type "Controller Object Reference") (DamageCauser :type "Actor Object Reference"))
  (bind _capsulecomponent (`self.CapsuleComponent`))
  (`SceneComponent.SetWorldScale3D` _capsulecomponent (+ (`SceneComponent.K2_GetComponentScale` _capsulecomponent) (0.1 0.1 0.1))))

(fn `SetAttackCooltime`
  (params (time :type "Float (double-precision)")))

(fn `TryAttack`
  (bind _returnvalue (`self.K2_GetActorLocation`))
  (bind _damage_radius (`self.Damage Radius`))
  (if (<= (`self.AttackCooltime`) 0.0)
    (`GameplayStatics.ApplyRadialDamage` :`BaseDamage` 5.0 :`Origin` _returnvalue :`DamageRadius` _damage_radius :`DamageCauser` null :`InstigatedByController` null)
    (`self.SetAttackCooltime` 1.0)
    (`KismetSystemLibrary.DrawDebugSphere` _returnvalue _damage_radius 12 (struct :`R` 1.0 :`A` 1.0) 1.0 2.0)))

(fn `Update Walk Speed`
  (params (NewWalkSpeed :type "Float (double-precision)"))
  (set `CharacterMovementComponent.MaxWalkSpeed` NewWalkSpeed (`self.CharacterMovement`)))

(fn `UserConstructionScript`)