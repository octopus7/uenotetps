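; Enemy cat character that periodically turns to face the player and fires a BP_BallYellowRed.
; Tick accumulates a cooldown timer; once it reaches the maximum, LookAndShoot snaps rotation toward the first actor tagged "Player" and spawns the ball ahead of the cat.
; The timer then keeps its overflow plus a small random offset, slightly varying the interval between shots.
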(event `self.ReceiveTick`
  (params (DeltaSeconds :type "Float (single-precision)"))
  (bind (_shootcooltime _shootcooltimemax _returnvalue) (`self.IsCoolTimeOver`))
  (if _returnvalue
    (`self.LookAndShoot`)
    (set `self.ShootCooltime` (+ (- _shootcooltime _shootcooltimemax) (`KismetMathLibrary.RandomFloatInRange` 0.0 0.1))))
  (set `self.ShootCooltime` (+ (`self.ShootCooltime`) DeltaSeconds)))

(fn `IsCoolTimeOver`
  (returns (ShootCooltime :type "Float (double-precision)") (ShootCooltimeMax :type "Float (double-precision)") (ReturnValue :type Boolean))
  (bind _shootcooltime (`self.ShootCooltime`))
  (bind _shootcooltimemax (`self.ShootCooltimeMax`))
  (return _shootcooltime _shootcooltimemax (>= _shootcooltime _shootcooltimemax)))

(fn `LookAndShoot`
  (bind (_returnvalue_location _returnvalue_rotation) (`KismetMathLibrary.BreakTransform` (`self.GetTransform`)))
  (bind _outactors (`GameplayStatics.GetAllActorsWithTag` "Player"))
  (`self.K2_SetActorRotation` (`KismetMathLibrary.FindLookAtRotation` (`self.K2_GetActorLocation`) (`self.K2_GetActorLocation` (`|GetArrayItem` _outactors))))
  (`|SpawnActorFromClass` "/Game/Blueprints/BP_BallYellowRed.BP_BallYellowRed_C" (`KismetMathLibrary.MakeTransform` (+ _returnvalue_location (* (`KismetMathLibrary.GetForwardVector` _returnvalue_rotation) 200.0)) _returnvalue_rotation) "Undefined" "MultiplyWithRoot" null null))

(fn `UserConstructionScript`)