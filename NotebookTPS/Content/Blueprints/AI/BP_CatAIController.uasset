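; BP_CatAIController is a cat AI controller that checks each Tick how far its pawn is from the Natsu player character.
; Beyond FollowThreshold it calls AIMoveTo, otherwise it stops movement.
; The move target and debug path goal are both the controlled pawn itself, not the player.
; Debug text shows the state and distance, and debug lines trace the navigation path on success.
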(event `self.ReceiveTick`
  (params (DeltaSeconds :type "Float (single-precision)"))
  (bind _returnvalue (`self.K2_GetPawn`))
  (bind _returnvalue_2 (`self.K2_GetActorLocation` (`self.K2_GetPawn`)))
  (bind _returnvalue_3 (`self.K2_GetActorLocation` _returnvalue))
  (bind _asbp_player_natsu (cast `/Game/Blueprints/BP_PlayerNatsu` (`GameplayStatics.GetPlayerCharacter` 0)))
  (bind _returnvalue_4 (`KismetMathLibrary.Vector_Distance` (`self.K2_GetActorLocation` _asbp_player_natsu) (`self.K2_GetActorLocation` (`self.K2_GetPawn`))))
  (if (> _returnvalue_4 (`self.FollowThreshold`))
    (`KismetSystemLibrary.DrawDebugString` _returnvalue_2 (`KismetStringLibrary.Concat_StrStr` "move" (`KismetStringLibrary.Conv_DoubleToString` (* (`KismetMathLibrary.Round` (* _returnvalue_4 10.0)) 0.1))) null (struct :`R` 1.0 :`G` 0.640301 :`A` 1.0))
    (`|AIMoveTo` (`self.K2_GetPawn`) (0.0 0.0 0.0) _returnvalue
      (:`then`
        (`KismetSystemLibrary.DrawDebugLine` _returnvalue_3 (`self.K2_GetActorLocation` _returnvalue) (struct :`R` 1.0 :`B` 0.645378 :`A` 1.0)))
      (:`OnSuccess`
        (bind _returnvalue_5 (`NavigationSystemV1.FindPathToActorSynchronously` (`NavigationSystemV1.GetNavigationSystem`) _returnvalue_3 _returnvalue 50.0 null null))
        (bind _pathpoints (`NavigationPath.PathPoints` _returnvalue_5))
        (for (_array_element _array_index) _pathpoints
          (if (> _array_index 0)
            (`KismetSystemLibrary.DrawDebugLine` (`|GetArrayItem` _pathpoints (- _array_index 1)) _array_element (struct :`R` 1.0 :`G` 0.635559 :`A` 1.0))))))
    (else
      (`KismetSystemLibrary.DrawDebugString` _returnvalue_2 "STOP" null (struct :`R` 1.0 :`G` 0.671533 :`B` 0.080851 :`A` 1.0))
      (`self.StopMovement`))))

(fn `UserConstructionScript`)